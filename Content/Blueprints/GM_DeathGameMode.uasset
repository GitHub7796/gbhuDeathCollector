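; GM_DeathGameMode is a game mode that tracks the player's scroll pickup score and converts it into a trophy tier.
; On BeginPlay it caches a GameInstance reference through a SetGIrefMessage call.
; AddScore increments and prints the score, while SetTroType maps score thresholds to one of three trophy enum values stored on the GameInstance.
; SetGamemodeRef returns the game mode itself as a reference.
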(event `self.ReceiveBeginPlay`
  ;[1 1 1] 获取GameInstance简化代码，后续引用
  (bind _gi (message `/Game/Blueprints/interfaces/INT_gameInstance.setGIref` (`GameplayStatics.GetGameInstance`)))
  (set `self.Gi` _gi))

(event `/Game/Blueprints/interfaces/INT_Gamemode.AddScore`
  ;[1 1 1] 每碰到卷轴，增加分数
  (bind _result (`/Engine/EditorBlueprintResources/StandardMacros.IncrementInt` (`self.score`))
    (:`  `
      (`KismetSystemLibrary.PrintString` (`KismetTextLibrary.Conv_TextToString` (`|FormatText` "you have {0} scores" _result))))))

(event `/Game/Blueprints/interfaces/INT_Gamemode.setTroType`
  (bind _score (`self.score`))
  (bind _gi (`self.Gi`))
  ;[1 1 1] 根据得分设置奖杯
  (if (<= _score 1)
    (set `/Game/Blueprints/GI_DeathCollector.Trophies` "NewEnumerator0" _gi)
    (elif (and (> _score 1) (<= _score 3))
      (set `/Game/Blueprints/GI_DeathCollector.Trophies` "NewEnumerator1" _gi)
      (else
        (set `/Game/Blueprints/GI_DeathCollector.Trophies` "NewEnumerator2" _gi)))))

(fn `setGamemodeRef`
  (returns (gameMode :type "/Game/Blueprints/GM_DeathGameMode Object Reference"))
  (return self))

(fn `UserConstructionScript`)