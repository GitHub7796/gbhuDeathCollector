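; BP_Scroll is a collectible scroll pickup that floats vertically and adds score when the player touches it.
; A timeline started on BeginPlay drives the Scroll component's relative Z for the bobbing motion.
; When an actor tagged "player" overlaps the Box, it waits briefly, adds score through message calls on the GameMode, plays a 2D sound and destroys itself.
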(event `self.ReceiveBeginPlay`
  ;[1 1 1] 上下自动浮动
  (bind (_direction _movement) (`Timeline|ScrollMovement` :!via `PlayFromStart`)
    (:`Update`
      (`SceneComponent.K2_SetRelativeLocation` (`self.scroll`) (`KismetMathLibrary.MakeVector` 0.0 0.0 (.z _movement)) false false))))

(event `self.Box.OnComponentBeginOverlap`
  (params (OverlappedComponent :type "PrimitiveComponent Object Reference") (OtherActor :type "Actor Object Reference") (OtherComp :type "PrimitiveComponent Object Reference") (OtherBodyIndex :type Integer) (bFromSweep :type Boolean) (SweepResult :type "HitResult Structure (by ref)"))
  ;[1 1 1] 被碰到后消失，新增分数，播放音乐
  (if (`self.ActorHasTag` OtherActor "player")
    (`KismetSystemLibrary.Delay` 0.2)
    (bind _gamemode (message `/Game/Blueprints/interfaces/INT_Gamemode.setGamemodeRef` (`GameplayStatics.GetGameMode`)))
    (message `/Game/Blueprints/interfaces/INT_Gamemode.AddScore` _gamemode)
    (`GameplayStatics.PlaySound2D` "/Game/Audio/SFX/SC_change_level.SC_change_level" 1.0 1.0 0.0 null null)
    (`self.K2_DestroyActor`)))

(fn `UserConstructionScript`)