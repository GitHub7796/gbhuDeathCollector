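; PC_DeathController is a controller that rolls the player pawn's ball from the MoveRight and MoveForward input axes.
; It gets the Ball component through the pawn's SetBallRefMessage call and applies scaled torque, around X for right and Y for forward.
; Each handler checks that the pawn is valid and retries after a short delay if not, guarding against errors when switching levels.
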(event `InputAxis|MoveRight`
  (params (AxisValue :type "Float (single-precision)"))
  (bind _returnvalue (`GameplayStatics.GetPlayerPawn` 0))
  ;[1 1 1] 左右移动
  ;;[1 1 1] 检验防止 切到新关卡报错
  (`/Engine/EditorBlueprintResources/StandardMacros.IsValid` _returnvalue :!label _label
    (:`Is Valid`
      (bind _ball (message `/Game/Blueprints/interfaces/INT_Ball.setBallRef` _returnvalue))
      (`PrimitiveComponent.AddTorqueInRadians` (`/Game/Maps/BP_Ball.ball` _ball) (`KismetMathLibrary.MakeVector` (* AxisValue 2000000.0)) "None" false))
    (:`Is Not Valid`
      (`KismetSystemLibrary.Delay` 0.2)
      (goto _label))))

(event `InputAxis|MoveForward`
  (params (AxisValue :type "Float (single-precision)"))
  (bind _returnvalue (`GameplayStatics.GetPlayerPawn` 0))
  ;[1 1 1] 上下移动
  (`/Engine/EditorBlueprintResources/StandardMacros.IsValid` _returnvalue :!label _label_2
    (:`Is Valid`
      (bind _ball (message `/Game/Blueprints/interfaces/INT_Ball.setBallRef` _returnvalue))
      (`PrimitiveComponent.AddTorqueInRadians` (`/Game/Maps/BP_Ball.ball` _ball) (`KismetMathLibrary.MakeVector` 0.0 (* AxisValue 2000000.0)) "None" false))
    (:`Is Not Valid`
      (`KismetSystemLibrary.Delay` 0.2)
      (goto _label_2))))

(fn `UserConstructionScript`)